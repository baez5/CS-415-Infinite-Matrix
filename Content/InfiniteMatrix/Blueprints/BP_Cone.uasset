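; BP_Cone is a hazard actor that damages the player on contact and can be shot for score.
; A hit on BP_Player decrements health, flags death and shows the restart display if health runs out, then destroys the cone.
; An overlapping BP_Projectile is always destroyed, but only a random one-in-three roll also destroys the cone and increments the instigating player's score.
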(event OnComponentHit(Cone)
  (params (HitComponent :type Primitive%20Component%20Object%20Reference) (OtherActor :type Actor%20Object%20Reference) (OtherComp :type Primitive%20Component%20Object%20Reference) (NormalImpulse :type Vector :default "0, 0, 0") (Hit :type Hit%20Result%20Structure%20%28by%20ref%29))
  (bind _asbp_player (Utilities|Casting|CastToBP_Player OtherActor))
  (bind _output_get (Default|DecrementHealth _asbp_player))
  (if (<= _output_get 0.0)
    (Variables|/Game/InfiniteMatrix/Blueprints/BP_Player.BP_Player_C|SetIsDead _asbp_player true)
    (Default|DisplayRestart _asbp_player)
    (Actor|DestroyActor)
    (else
      (Actor|DestroyActor))))

(event OnComponentBeginOverlap(Cone)
  (params (OverlappedComponent :type Primitive%20Component%20Object%20Reference) (OtherActor :type Actor%20Object%20Reference) (OtherComp :type Primitive%20Component%20Object%20Reference) (OtherBodyIndex :type Integer) (bFromSweep :type Boolean) (SweepResult :type Hit%20Result%20Structure%20%28by%20ref%29))
  (bind _asbp_projectile (Utilities|Casting|CastToBP_Projectile OtherActor))
  (if (== 1 (Math|Random|RandomIntegerinRange 0 2))
    (Actor|DestroyActor)
    (bind _asbp_player (Utilities|Casting|CastToBP_Player (Game|GetInstigator _asbp_projectile)))
    (Default|IncrementScore _asbp_player)
    (Actor|DestroyActor _asbp_projectile)
    (else
      (Actor|DestroyActor _asbp_projectile))))

(event EventBeginPlay)

(event Collision|EventActorBeginOverlap
  (params (OtherActor :type Actor%20Object%20Reference)))

(event EventTick
  (params (DeltaSeconds :type Float%20%28single-precision%29)))

(fn ConstructionScript)